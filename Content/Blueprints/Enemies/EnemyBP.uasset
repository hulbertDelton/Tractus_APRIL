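; Enemy that flies toward the first DemoPlanetBP found at spawn, turning to face it and drawing a debug arrow along its path.
; FloatingPawnMovement drives the approach each tick, pausing during timed stuns, while a separate KbEnemyMovement component takes knockback.
; Damage lowers HP and updates a health widget; at zero the enemy destroys itself and awards money through TractusPlayerController.
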(event Custom|EndStun
  (Variables|Default|SetisStunned false))

(event Custom|Event%20Knockback%20Damage
  (params (KnockbackVector :type Vector))
  (Class|PawnMovementComponent|AddInputVector (Variables|Default|GetkbEnemyMovement) KnockbackVector false))

(event EventBeginPlay
  (CallFunction|TurntoTarget)
  (CallFunction|FindTargetPlanet)
  (CallFunction|SetupHpWidget)
  (Default|UpdateHealth (Variables|Default|GetHpWidgetRef) (Variables|Default|GetHp)))

(event Collision|EventActorBeginOverlap
  (params (OtherActor :type Actor%20Object%20Reference)))

(event EventTick
  (params (DeltaSeconds :type Float%20%28single-precision%29))
  (CallFunction|MovetoTarget))

(event Game|Damage|EventAnyDamage
  (params (Damage :type Float%20%28single-precision%29) (DamageType :type Damage%20Type%20Object%20Reference) (InstigatedBy :type Controller%20Object%20Reference) (DamageCauser :type Actor%20Object%20Reference))
  (bind _output_get (Variables|Default|SetHp (- (Variables|Default|GetHp) Damage)))
  (if (<= _output_get 0.0)
    (Actor|DestroyActor)
    (bind _astractus_player_controller (Utilities|Casting|CastToTractusPlayerController (Game|GetPlayerController 0))
      (:then
        (Default|UpdateMoney _astractus_player_controller 75))
      (:CastFailed
        (Development|PrintString "Error unable to grant money")))
    (else
      (Default|UpdateHealth (Variables|Default|GetHpWidgetRef) (Variables|Default|GetHp)))))

(event EventDestroyed)

(event EventKnockback
  (params (Direction :type Vector :default "0, 0, 0"))
  (Variables|/Script/Engine.MovementComponent|SetVelocity (Variables|Default|GetkbEnemyMovement) Direction))

(event EventStun
  (params (Duration :type Float%20%28single-precision%29))
  (Utilities|Time|SetTimerbyEvent (delegate Custom|EndStun) Duration)
  (Variables|Default|SetisStunned true)
  (Variables|/Script/Engine.MovementComponent|SetVelocity (Variables|Default|GetFloatingPawnMovement) "0, 0, 0"))

(fn ConstructionScript)

(fn TurntoTarget
  (Transformation|SetActorRotation (Math|Rotator|CombineRotators "90.000000, 0,90.000000" (Math|Rotator|MakeRotfromZ (- (Variables|Default|GetTargetCoords) (Transformation|GetActorLocation))))))

(fn FindTargetPlanet
  (bind _outactors (Actor|GetAllActorsOfClass "/Game/Blueprints/DemoPlanetBP.DemoPlanetBP_C"))
  (bind _output_get (Variables|Default|SetTargeted%20planet (Utilities|Array|Get(acopy) _outactors)))
  (Variables|Default|SetTargetCoords (Transformation|GetActorLocation _output_get)))

(fn OnRepKnockback)

(fn SetupHpWidget
  (bind _ashp_widget_bp (Utilities|Casting|CastToHpWidgetBP (UserInterface|GetUserWidgetObject (Variables|Default|GetHpWidget))))
  (Variables|Default|SetHpWidgetRef _ashp_widget_bp))

(fn MovetoTarget
  (bind _returnvalue (Transformation|GetActorLocation))
  (bind _targetcoords (Variables|Default|GetTargetCoords))
  (CallFunction|TurntoTarget)
  (if (not (Variables|Default|GetisStunned))
    (Class|PawnMovementComponent|AddInputVector (Variables|Default|GetFloatingPawnMovement) (- _targetcoords _returnvalue) false)
    (Rendering|Debug|DrawDebugArrow _returnvalue _targetcoords 4e+02 "(R=0.085906,G=0.161458,B=0.016779,A=0.504000)" 0.0 5.0)))