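; Enemy formation actor, centred on the first DemoPlanetBP, that spawns EnemyBP units and leads them along a spline.
; A looping timer spawns units at the spline's end, adding a static mesh component for each, until the set count is reached.
; Each tick a sphere moves backward along the spline at enemy max speed, serving as every unit's target.
; The formation destroys itself once the destroyed count reaches the unit total.
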(event Custom|HandleDestroyedUnit
  (params (DestroyedUnit :type Actor%20Object%20Reference))
  (Math|Integer|IncrementInt (Variables|Default|GetNumUnitsDestroyed)))

(event EventBeginPlay
  (CallFunction|ResetSpherePosition)
  (Utilities|Time|SetTimerbyFunctionName 0 "AddEnemies" 1.0 true))

(event Collision|EventActorBeginOverlap
  (params (OtherActor :type Actor%20Object%20Reference)))

(event EventTick
  (params (DeltaSeconds :type Float%20%28single-precision%29))
  (CallFunction|MoveSphereAlongSpline DeltaSeconds)
  (bind _isvalid (CallFunction|CheckifUnitsAreDestroyed))
  (if _isvalid
    (for _array_element (Variables|Default|GetUnitsInFormation)
      (Utilities|IsValid _array_element
        (:Is%20Valid
          (Variables|/Game/Blueprints/Enemies/EnemyBP.EnemyBP_C|SetTargetCoords _array_element (Transformation|GetWorldLocation (Variables|Default|GetSphere))))))))

(fn ConstructionScript
  (if (Utilities|IsValid (Variables|Default|GetInputSpline))
    (Variables|Default|SetSpline (Variables|Default|GetInputSpline)))
  (bind _outactors (Actor|GetAllActorsOfClass "/Game/Blueprints/DemoPlanetBP.DemoPlanetBP_C"))
  (Transformation|SetWorldLocation (Variables|Default|GetDefaultSceneRoot) (Transformation|GetActorLocation (Utilities|Array|Get(acopy) _outactors)) false false))

(fn MoveSphereAlongSpline
  (params (DeltaSeconds :type Float%20%28single-precision%29))
  (bind _totaltimeelapsed (CallFunction|AccumulateTime DeltaSeconds false))
  (Transformation|SetRelativeTransform (Variables|Default|GetSphere) (Spline|GetTransformatDistanceAlongSpline (Variables|Default|GetSpline) (- (Spline|GetSplineLength (Variables|Default|GetSpline)) (* _totaltimeelapsed (Variables|Default|GetMovement%20Speed))) "Local" true) false false))

(fn ResetSpherePosition
  (bind _spline (Variables|Default|GetSpline))
  (Transformation|SetRelativeLocation (Variables|Default|GetSphere) (.Location (Math|Transform|BreakTransform (Spline|GetTransformatSplinePoint _spline (Spline|GetNumberOfSplinePoints _spline) "Local" false))) false false))

(fn AccumulateTime
  (params (DeltaSeconds :type Float%20%28single-precision%29) (Reset :type Boolean))
  (if Reset
    (Variables|Default|SetTimeElapsed 0.0))
  (bind _output_get (Variables|Default|SetTimeElapsed (+ DeltaSeconds (Variables|Default|GetTimeElapsed))))
  (return _output_get))

(fn AddEnemies
  (bind _spline (Variables|Default|GetSpline))
  (bind _returnvalue (Spline|GetNumberOfSplinePoints _spline))
  (bind _returnvalue_2 (Spline|GetTransformatSplinePoint _spline _returnvalue "World" false))
  (bind _returnvalue_3 (Game|SpawnActorfromClass "/Game/Blueprints/Enemies/EnemyBP.EnemyBP_C" _returnvalue_2 "AlwaysSpawn" self 0))
  (bind _returnvalue_4 (AddComponent|AddStaticMeshComponent false _returnvalue_2))
  (Transformation|AddLocalOffset _returnvalue_4 "0, 0,-50.000000" false false)
  (Utilities|Array|Add (Variables|Default|GetUnit%20Leaders) _returnvalue_4)
  (Game|BindEventtoOnDestroyed _returnvalue_3 (EventDispatchers|CreateEvent :!event Custom|HandleDestroyedUnit))
  (Utilities|Array|Add (Variables|Default|GetUnitsInFormation) _returnvalue_3)
  (Variables|Default|SetMovement%20Speed (Variables|/Script/Engine.FloatingPawnMovement|GetMaxSpeed (Variables|/Game/Blueprints/Enemies/EnemyBP.EnemyBP_C|GetFloatingPawnMovement _returnvalue_3)))
  (bind _result (Math|Integer|IncrementInt (Variables|Default|GetUnitsSpawned))
    (:%20%20
      (if (== _result (Variables|Default|GetUnits))
        (Utilities|Time|ClearTimerbyFunctionName 0 "AddEnemies")))))

(fn CheckifUnitsAreDestroyed
  (if (< (Variables|Default|GetNumUnitsDestroyed) (Variables|Default|GetUnits))
    (return true)
    (else
      (Actor|DestroyActor)
      (return false))))

(fn CleanupFormation
  (for _array_element (Variables|Default|GetUnitsInFormation)
    (Utilities|IsValid _array_element
      (:Is%20Not%20Valid
        (Utilities|Array|RemoveItem (Variables|Default|GetUnitsInFormation) 0)
        (Math|Integer|IncrementInt (Variables|Default|GetNumUnitsDestroyed))))))