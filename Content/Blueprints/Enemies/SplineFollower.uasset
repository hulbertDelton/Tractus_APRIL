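; Spline path helper in the Enemies folder that supplies a target location for following a spline, without moving anything itself.
; UpdatePosition advances the point index when the given location is within the acceptance threshold and records the distance to the next point.
; The returned target slides from the current point toward the following one as that distance shrinks, leading the follower around corners.
; Each call draws a debug circle at the current point.
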(event EventBeginPlay)

(event Collision|EventActorBeginOverlap
  (params (OtherActor :type Actor%20Object%20Reference)))

(event EventTick
  (params (DeltaSeconds :type Float%20%28single-precision%29)))

(fn ConstructionScript)

(fn UpdatePosition
  (params (AcceptanceThreshold :type Float%20%28single-precision%29) (CurrentLocation :type Vector))
  (bind _spline (Variables|Default|GetSpline))
  (bind _idx (Variables|Default|Getidx))
  (bind _returnvalue (Spline|GetLocationatSplinePoint _spline _idx "World"))
  (LocalVariables|SetCurrentLocation_ CurrentLocation)
  (if (<= (Variables|Default|GetMaxLengthtoNextPoint) 0.0)
    (Variables|Default|SetMaxLengthtoNextPoint (Math|Vector|VectorLength (- (Spline|GetLocationatSplinePoint (Variables|Default|GetSpline) (Variables|Default|Getidx) "World") (LocalVariables|GetCurrentLocation_)))))
  (Rendering|Debug|DrawDebugCircle _returnvalue AcceptanceThreshold 12 "(R=1.000000,G=1.000000,B=1.000000,A=1.000000)" 1.0 0.0 "0.000000,1.000000,0.000000" "1.000000,0.000000,0.000000")
  (if (< (Math|Vector|VectorLength (- _returnvalue (LocalVariables|GetCurrentLocation_))) AcceptanceThreshold)
    (bind _result (Math|Integer|IncrementInt (Variables|Default|Getidx))
      (:%20%20
        (Variables|Default|SetMaxLengthtoNextPoint (Math|Vector|VectorLength (- (Spline|GetLocationatSplinePoint (Variables|Default|GetSpline) _result "World") (LocalVariables|GetCurrentLocation_)))))))
  (return (+ (* (- (Spline|GetLocationatSplinePoint (Variables|Default|GetSpline) (+ (Variables|Default|Getidx) 1) "World") _returnvalue) (- 1.0 (/ (Math|Vector|VectorLength (- _returnvalue (LocalVariables|GetCurrentLocation_))) (Variables|Default|GetMaxLengthtoNextPoint)))) _returnvalue)))