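; Enemy formation actor that spawns a wave of EnemyBP units along a spline path and tracks their destruction.
; A looping timer spawns each enemy with an invisible-to-logic SplineFollower leader, mapped in UnitLeaders; Tick feeds the leader's updated position into each enemy's TargetCoords.
; Destroyed enemies remove their leader and increment the count CheckForExit compares against Units.
; Construction builds colored spline meshes, or snaps to DemoPlanetBP without a spline.
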(event Custom|CustomEventOnDestoryed)

(event Custom|HandleDestroyedUnit
  (params (DestroyedUnit :type Actor%20Object%20Reference))
  (bind _asenemy_bp (Utilities|Casting|CastToEnemyBP DestroyedUnit))
  (Actor|DestroyActor (.Value (Utilities|Map|Find (Variables|Default|GetUnit%20Leaders) _asenemy_bp)))
  (Utilities|Map|Remove (Variables|Default|GetUnit%20Leaders) _asenemy_bp)
  (Math|Integer|IncrementInt (Variables|Default|GetNumUnitsDestroyed)))

(event EventBeginPlay
  (Utilities|Time|SetTimerbyFunctionName 0 "BeginSpawningEnemies" 1.0 true))

(event Collision|EventActorBeginOverlap
  (params (OtherActor :type Actor%20Object%20Reference)))

(event EventTick
  (params (DeltaSeconds :type Float%20%28single-precision%29))
  (CallFunction|UpdateEnemyLocations))

(fn ConstructionScript
  (if (Utilities|IsValid (Variables|Default|GetInputSpline))
    (CallFunction|ConstructSplineActor)
    (else
      (bind _outactors (Actor|GetAllActorsOfClass "/Game/Blueprints/DemoPlanetBP.DemoPlanetBP_C"))
      (Transformation|SetWorldLocation (Variables|Default|GetDefaultSceneRoot) (Transformation|GetActorLocation (Utilities|Array|Get(acopy) _outactors)) false false))))

(fn BeginSpawningEnemies
  (bind _inputspline (Variables|Default|GetInputSpline))
  (bind _returnvalue (Spline|GetLocationatSplinePoint _inputspline 0 "World"))
  (bind _returnvalue_2 (Math|Transform|MakeTransform _returnvalue))
  (if (>= (Variables|Default|GetUnitsSpawned) (Variables|Default|GetUnits))
    (Utilities|Time|ClearTimerbyFunctionName 0 "BeginSpawningEnemies")
    (else
      (Math|Integer|IncrementInt (Variables|Default|GetUnitsSpawned)
        (:%20%20
          (bind _returnvalue_3 (Game|SpawnActorfromClass "/Game/Blueprints/Enemies/SplineFollower.SplineFollower_C" _returnvalue_2 "Undefined" 0 (Variables|Default|GetInputSpline) 0))
          (bind _returnvalue_4 (Game|SpawnActorfromClass "/Game/Blueprints/Enemies/EnemyBP.EnemyBP_C" _returnvalue_2 "Undefined" 0 0))
          (Utilities|Map|Add (Variables|Default|GetUnit%20Leaders) _returnvalue_4 _returnvalue_3)
          (Game|BindEventtoOnDestroyed _returnvalue_4 (EventDispatchers|CreateEvent :!event Custom|HandleDestroyedUnit)))))))

(fn UpdateEnemyLocations
  (bind _unit_leaders (Variables|Default|GetUnit%20Leaders))
  (bind _keys (Utilities|Map|Keys _unit_leaders))
  (for _array_element _keys
    (bind _targetlocation (Default|UpdatePosition (.Value (Utilities|Map|Find _unit_leaders _array_element)) 1e+02 (Transformation|GetWorldLocation (Variables|/Script/Engine.Actor|GetRootComponent _array_element))))
    (Variables|/Game/Blueprints/Enemies/EnemyBP.EnemyBP_C|SetTargetCoords _array_element _targetlocation)))

(fn CheckforExit
  (if (== (Variables|Default|GetUnits) (Variables|Default|GetNumUnitsDestroyed))
    (return true)
    (else
      (return false))))

(fn ConstructSplineActor
  (bind _inputspline (Variables|Default|GetInputSpline))
  (for _index (range 0 (- (Spline|GetNumberOfSplinePoints (Variables|Default|GetInputSpline)) 2))
    (bind _returnvalue (AddComponent|AddSplineMeshComponent false))
    (Components|StaticMesh|SetStaticMesh _returnvalue (Variables|Default|GetSplineMesh))
    (bind _returnvalue_2 (Rendering|Material|CreateDynamicMaterialInstance (Variables|Default|GetMaterial) "Name" :!class /Script/Engine.KismetMaterialLibrary))
    (Rendering|Material|SetVectorParameterValue _returnvalue_2 "Color" (Variables|Default|GetColor) :!class /Script/Engine.MaterialInstanceDynamic)
    (Rendering|Material|SetMaterial _returnvalue 0 _returnvalue_2)
    (SplineMesh|SetForwardAxis _returnvalue (Variables|Default|GetForwardAxis) true)
    (Transformation|AttachComponentToComponent _returnvalue (Variables|Default|GetInputSpline) "None" "KeepRelative" "KeepRelative" "KeepRelative" true)
    (SplineMesh|SetStartandEnd _returnvalue (.Location (Spline|GetLocationandTangentatSplinePoint _inputspline _index "Local")) (.Tangent (Spline|GetLocationandTangentatSplinePoint _inputspline _index "Local")) (.Location (Spline|GetLocationandTangentatSplinePoint _inputspline (+ _index 1) "Local")) (.Tangent (Spline|GetLocationandTangentatSplinePoint _inputspline (+ _index 1) "Local")) true :!class /Script/Engine.SplineMeshComponent)))