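; Player planet that destroys any actor overlapping its hitbox, accumulates damage and passes money totals to the HUD.
; The construction script builds concentric rings, each larger one gaining a turret socket and getting an inverse-square slower rotation speed.
; Sockets are evenly spaced around each ring, each owning a Paper sprite as its selection interface.
; Alternative child-actor and widget socket builders exist, but construction uses only the sprite path.
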(event Custom|CustomEvent_0
  (params (OverlappedComponent :type Primitive%20Component%20Object%20Reference) (OtherActor :type Actor%20Object%20Reference) (OtherComp :type Primitive%20Component%20Object%20Reference) (OtherBodyIndex :type Integer) (bFromSweep :type Boolean) (SweepResult :type Hit%20Result%20Structure%20%28by%20ref%29))
  (Development|PrintString (Utilities|GetDisplayName OtherActor))
  (Actor|DestroyActor OtherActor)
  (CallFunction|DoDamage 1))

(event Custom|DestroyEnemy
  (params (OverlappedComponent :type Primitive%20Component%20Object%20Reference) (OtherActor :type Actor%20Object%20Reference) (OtherComp :type Primitive%20Component%20Object%20Reference) (OtherBodyIndex :type Integer) (bFromSweep :type Boolean) (SweepResult :type Hit%20Result%20Structure%20%28by%20ref%29)))

(event EventBeginPlay
  (Collision|BindEventtoOnComponentBeginOverlap (Variables|Default|GetHitbox) (delegate Custom|CustomEvent_0))
  (CallFunction|SetupPlayerController))

(event Collision|EventActorBeginOverlap
  (params (OtherActor :type Actor%20Object%20Reference)))

(event EventTick
  (params (DeltaSeconds :type Float%20%28single-precision%29)))

(fn ConstructionScript
  (CallFunction|ConstructRingsasSprites (Variables|Default|GetNumRings)))

(fn DoDamage
  (params (DamageAmount :type Integer))
  (Variables|Default|SetDamage (+ DamageAmount (Variables|Default|GetDamage))))

(fn CalculateSize
  (params (index :type Integer))
  (return (+ (* index (Variables|Default|GetDistanceBetweenRings)) (Variables|Default|GetBaseRingSize))))

(fn ConstructTurretSockets
  (params (TargetRing :type Ring%20BP%20Object%20Reference))
  (bind _numturrets (Variables|/Game/Blueprints/RingBP.RingBP_C|GetNumTurrets TargetRing))
  (LocalVariables|SetActiveRing TargetRing)
  (for _index (range 1 _numturrets)
    (bind _newparam2 (Default|AnglefromIndex (LocalVariables|GetActiveRing) _index _numturrets))
    (bind _returnvalue (AddComponent|AddChildActorComponent true (Math|Conversions|ToTransform(Vector) (Math|Vector|RotateVector (Math|Vector|MakeVector (Variables|/Game/Blueprints/RingBP.RingBP_C|GetSize TargetRing) 0.0 0.0) (Math|Rotator|MakeRotator 0.0 0.0 _newparam2)))))
    (Transformation|SetRelativeRotation _returnvalue (Math|Rotator|MakeRotator 0.0 0.0 _newparam2) false false)
    (bind _asturret_socket_actor (Utilities|Casting|CastToTurretSocketActor (Variables|/Script/Engine.ChildActorComponent|GetChildActor _returnvalue)))
    (Variables|/Game/Blueprints/TurretSocketActor.TurretSocketActor_C|SetMyRing _asturret_socket_actor (LocalVariables|GetActiveRing))
    (Transformation|AttachComponentToComponent _returnvalue (LocalVariables|GetActiveRing) "None" "KeepRelative" "KeepRelative" "KeepWorld" false)))

(fn ConstructTurretasActor
  (params (TargetRing :type Ring%20BP%20Object%20Reference))
  (bind _numturrets (Variables|/Game/Blueprints/RingBP.RingBP_C|GetNumTurrets TargetRing))
  (for _index (range 1 _numturrets)
    (bind _newparam2 (Default|AnglefromIndex TargetRing _index _numturrets))
    (bind _returnvalue (AddComponent|AddChildActorComponent false (Math|Conversions|ToTransform(Vector) (Math|Vector|RotateVector (Math|Vector|MakeVector (Variables|/Game/Blueprints/RingBP.RingBP_C|GetSize TargetRing) 0.0 0.0) (Math|Rotator|MakeRotator 0.0 0.0 _newparam2)))))
    (Transformation|SetRelativeScale3D _returnvalue "0.500000,0.500000,0.500000")
    (Transformation|AttachComponentToComponent _returnvalue TargetRing "None" "KeepRelative" "KeepRelative" "KeepRelative" false)
    (bind _asturret_actor (Utilities|Casting|CastToTurretActor (Variables|/Script/Engine.ChildActorComponent|GetChildActor _returnvalue)))
    (Variables|/Game/Blueprints/Turrets/TurretActor.TurretActor_C|SetParentPlanet _asturret_actor self)))

(fn AddMoney
  (params (amount :type Integer))
  (bind _output_get (Variables|Default|SetMoney (+ amount (Variables|Default|GetMoney))))
  (Default|SetMoney (Variables|/Game/Blueprints/TractusPlayerController.TractusPlayerController_C|GetHUD (Variables|Default|GetMyController)) _output_get))

(fn SetupPlayerController
  (bind _astractus_player_controller (Utilities|Casting|CastToTractusPlayerController (Pawn|GetController)))
  (Variables|Default|SetMyController _astractus_player_controller))

(fn ConstructRings
  (params (LastIndex :type Integer))
  (for _index (range 1 LastIndex)
    (bind _size (CallFunction|CalculateSize _index))
    (bind _returnvalue (AddComponent|AddRingBP true (Math|Transform|MakeTransform "0, 0, 0") _size (+ _index 3) (/ 2e+05 (* _size _size))))
    (Utilities|Array|Add (Variables|Default|Getrings) _returnvalue)
    (Transformation|AttachComponentToComponent _returnvalue (Variables|Transformation|GetRootComponent) "None" "KeepRelative" "KeepRelative" "KeepWorld" true)
    (Default|Draw _returnvalue)
    (CallFunction|ConstructTurretSockets _returnvalue)))

(fn ConstructRingsasWidgets
  (params (LastIndex :type Integer))
  (for _index (range 1 LastIndex)
    (bind _size (CallFunction|CalculateSize _index))
    (bind _returnvalue (AddComponent|AddRingBP true (Math|Transform|MakeTransform "0, 0, 0") _size (+ _index 3) (/ 2e+05 (* _size _size))))
    (Utilities|Array|Add (Variables|Default|Getrings) _returnvalue)
    (Transformation|AttachComponentToComponent _returnvalue (Variables|Transformation|GetRootComponent) "None" "KeepRelative" "KeepRelative" "KeepWorld" true)
    (Default|Draw _returnvalue)
    (CallFunction|ConstructTurretSocketsasWidgets _returnvalue)))

(fn ConstructTurretSocketsasWidgets
  (params (TargetRing :type Ring%20BP%20Object%20Reference))
  (bind _numturrets (Variables|/Game/Blueprints/RingBP.RingBP_C|GetNumTurrets TargetRing))
  (LocalVariables|SetActiveRing TargetRing)
  (for _index (range 1 _numturrets)
    (bind _newparam2 (Default|AnglefromIndex (LocalVariables|GetActiveRing) _index _numturrets))
    (bind _returnvalue (AddComponent|AddTurretSocketBase false (Math|Conversions|ToTransform(Vector) (Math|Vector|RotateVector (Math|Vector|MakeVector (Variables|/Game/Blueprints/RingBP.RingBP_C|GetSize TargetRing) 0.0 0.0) (Math|Rotator|MakeRotator 0.0 0.0 _newparam2)))))
    (Transformation|SetRelativeRotation _returnvalue (Math|Rotator|MakeRotator 0.0 0.0 _newparam2) false false)
    (Transformation|AttachComponentToComponent _returnvalue (LocalVariables|GetActiveRing) "None" "KeepRelative" "KeepRelative" "KeepRelative" false)
    (CallFunction|AddWidget (Math|Conversions|ToTransform(Vector) (Math|Vector|RotateVector (Math|Vector|MakeVector (Variables|/Game/Blueprints/RingBP.RingBP_C|GetSize TargetRing) 0.0 0.0) (Math|Rotator|MakeRotator 0.0 0.0 _newparam2))) _returnvalue)))

(fn AddWidget
  (params (RelativeTransform :type Transform) (AttachTarget :type Scene%20Component%20Object%20Reference))
  (bind _returnvalue (AddComponent|AddWidgetComponent false))
  (Transformation|AttachComponentToComponent _returnvalue AttachTarget "None" "KeepRelative" "KeepWorld" "KeepWorld" false)
  (Transformation|SetRelativeRotation _returnvalue "90.000000, 0, 0" false false)
  (CallFunction|SetSocketinWidget _returnvalue AttachTarget))

(fn SetSocketinWidget
  (params (self2 :type Widget%20Component%20Object%20Reference) (Object :type Object%20Object%20Reference))
  (bind _asselector_bp (Utilities|Casting|CastToSelectorBP (UserInterface|GetUserWidgetObject self2))
    (:then
      (bind _asturret_socket_base (Utilities|Casting|CastToTurretSocketBase Object)
        (:then
          (Variables|/Game/UserInterface/turretUI/SelectorBP.SelectorBP_C|SetParent%20Socket _asselector_bp _asturret_socket_base))
        (:CastFailed
          (Development|PrintString "cast failed" :!label _label))))
    (:CastFailed
      (goto _label))))

(fn ConstructRingsasSprites
  (params (LastIndex :type Integer))
  (for _index (range 1 LastIndex)
    ;[1 1 1] Build A Ring
    (bind _size (CallFunction|CalculateSize _index))
    (bind _returnvalue (AddComponent|AddRingBP true (Math|Transform|MakeTransform "0, 0, 0") _size (+ _index 3) (/ 2e+05 (* _size _size))))
    (Utilities|Array|Add (Variables|Default|Getrings) _returnvalue)
    (Transformation|AttachComponentToComponent _returnvalue (Variables|Transformation|GetRootComponent) "None" "KeepRelative" "KeepRelative" "KeepWorld" true)
    (Default|Draw _returnvalue)
    (CallFunction|ConstructTurretSocketsasSprites _returnvalue)))

(fn ConstructTurretSocketsasSprites
  (params (TargetRing :type Ring%20BP%20Object%20Reference))
  (bind _numturrets (Variables|/Game/Blueprints/RingBP.RingBP_C|GetNumTurrets TargetRing))
  (LocalVariables|SetActiveRing TargetRing)
  (for _index (range 1 _numturrets)
    (bind _newparam2 (Default|AnglefromIndex (LocalVariables|GetActiveRing) _index _numturrets))
    (bind _returnvalue (AddComponent|AddTurretSocketBase false (Math|Conversions|ToTransform(Vector) (Math|Vector|RotateVector (Math|Vector|MakeVector (Variables|/Game/Blueprints/RingBP.RingBP_C|GetSize TargetRing) 0.0 0.0) (Math|Rotator|MakeRotator 0.0 0.0 _newparam2)))))
    (Transformation|SetRelativeRotation _returnvalue (Math|Rotator|MakeRotator 0.0 0.0 _newparam2) false false)
    (Transformation|AttachComponentToComponent _returnvalue (LocalVariables|GetActiveRing) "None" "KeepRelative" "KeepRelative" "KeepRelative" false)
    (bind _sprite (CallFunction|AddSprite (Math|Conversions|ToTransform(Vector) (Math|Vector|RotateVector (Math|Vector|MakeVector (Variables|/Game/Blueprints/RingBP.RingBP_C|GetSize TargetRing) 0.0 0.0) (Math|Rotator|MakeRotator 0.0 0.0 _newparam2))) _returnvalue))
    (Variables|/Game/Blueprints/TurretSocketBase.TurretSocketBase_C|SetOwnedSelectionInterface _returnvalue _sprite)))

(fn AddSprite
  (params (RelativeTransform :type Transform) (AttachTarget :type Scene%20Component%20Object%20Reference))
  (bind _returnvalue (AddComponent|AddPaperSpriteComponent true))
  (Transformation|AttachComponentToComponent _returnvalue AttachTarget "None" "KeepRelative" "KeepWorld" "KeepWorld" false)
  (Transformation|SetRelativeRotation _returnvalue "0.000000,0.000000,90.000000" false false)
  (return _returnvalue))