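; Satellite actor that carries a ring of turret sockets, with a TurretOrientation component that rotates a fixed step every tick.
; The construction script spaces sockets by angle around RingBP, using its turret count and size, and attaches them to it.
; Each socket gets a rotated Paper2D sprite stored as its selection interface.
; When the satellite is destroyed, it calls DestroyTurret on every owned socket.
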(event EventBeginPlay
  (|CallParentFunction) ; This node is disabled and will not be called.\nDrag off pins to build functionality.
)

(event Collision|EventActorBeginOverlap
  (params (OtherActor :type Actor%20Object%20Reference))
  (|CallParentFunction OtherActor) ; This node is disabled and will not be called.\nDrag off pins to build functionality.
)

(event EventTick
  (params (DeltaSeconds :type Float%20%28single-precision%29))
  (Transformation|AddLocalRotation (Variables|Default|GetTurretOrientation) "0,-1.000000, 0" false false))

(event EventDestroyed
  (Development|PrintString "InSatelliteShutdown")
  (for _array_element (Variables|Default|GetOwnedSockets)
    (Default|DestroyTurret _array_element)
    (Development|PrintString "Hello")))

(fn ConstructionScript
  (|CallParentFunction)
  (CallFunction|ConstructRingsasSprites (Variables|Default|GetRingBP)))

(fn ConstructRingsasSprites
  (params (NewParam :type Ring%20BP%20Object%20Reference))
  (bind _numturrets (Variables|/Game/Blueprints/RingBP.RingBP_C|GetNumTurrets NewParam))
  (LocalVariables|SetActiveRing NewParam)
  (for _index (range 1 _numturrets)
    (bind _newparam2 (Default|AnglefromIndex (LocalVariables|GetActiveRing) _index _numturrets))
    (bind _returnvalue (AddComponent|AddTurretSocketBase false (Math|Conversions|ToTransform(Vector) (Math|Vector|RotateVector (Math|Vector|MakeVector (Variables|/Game/Blueprints/RingBP.RingBP_C|GetSize NewParam) 0.0 0.0) (Math|Rotator|MakeRotator 0.0 0.0 _newparam2)))))
    (Utilities|Array|Add (Variables|Default|GetOwnedSockets) _returnvalue)
    (Transformation|SetRelativeRotation _returnvalue (Math|Rotator|MakeRotator 0.0 0.0 _newparam2) false false)
    (Transformation|AttachComponentToComponent _returnvalue (LocalVariables|GetActiveRing) "None" "KeepRelative" "KeepRelative" "KeepRelative" false)
    (bind _sprite (CallFunction|AddSprite _returnvalue))
    (Variables|/Game/Blueprints/TurretSocketBase.TurretSocketBase_C|SetOwnedSelectionInterface _returnvalue _sprite)))

(fn AddSprite
  (params (AttachTarget :type Scene%20Component%20Object%20Reference))
  (bind _returnvalue (AddComponent|AddPaperSpriteComponent true))
  (Transformation|AttachComponentToComponent _returnvalue AttachTarget "None" "KeepRelative" "KeepWorld" "KeepWorld" false)
  (Transformation|SetRelativeRotation _returnvalue "0.000000,0.000000,90.000000" false false)
  (return _returnvalue))