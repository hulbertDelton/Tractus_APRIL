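; Virus turret projectile, a child Blueprint that spreads like an infection by spawning copies of itself when it damages an enemy.
; On hit, ReTarget sphere-traces within DamageRadius, ignoring the struck enemy, and spawns a projectile aimed at each hit's impact point.
; An incremented Iteration counter caps the branching chain at three generations.
; The parent handles damage, while this class adds attached fire VFX, impact VFX and hit sound.
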(event EventBeginPlay
  (|CallParentFunction)
  (Effects|SpawnEmitterAttached "/Game/VFX/weaponEffects/virus/virus_fireVFX_ver01.virus_fireVFX_ver01" (Variables|Default|GetBox) "None"))

(event Collision|EventActorBeginOverlap
  (params (OtherActor :type Actor%20Object%20Reference))
  (|CallParentFunction OtherActor) ; This node is disabled and will not be called.\nDrag off pins to build functionality.
)

(event EventTick
  (params (DeltaSeconds :type Float%20%28single-precision%29))
  (|CallParentFunction DeltaSeconds) ; This node is disabled and will not be called.\nDrag off pins to build functionality.
)

(event EventDamageEnemy
  (params (DamagedActor :type Actor%20Object%20Reference))
  (bind _returnvalue (Transformation|GetActorTransform))
  (bind (_location _rotation) (Math|Transform|BreakTransform _returnvalue))
  (CallFunction|ReTarget DamagedActor)
  (|CallParentFunction DamagedActor)
  (Effects|SpawnEmitteratLocation "/Game/VFX/weaponEffects/virus/virus_impactVFX_ver01.virus_impactVFX_ver01" _location _rotation "1.000000,1.000000,1.000000" false "AutoRelease")
  (Audio|SpawnSoundatLocation "/Game/SFX/testingSounds/Turrets/SPEAR_Hit.SPEAR_Hit" _location "0, 0, 0" 1.0 1.0 0.0 0 0))

(fn ConstructionScript
  (|CallParentFunction))

(fn ReTarget
  (params (EnemyHit :type Actor%20Object%20Reference))
  (bind _returnvalue (Transformation|GetActorLocation))
  (if (< (Variables|Default|GetIteration) 3)
    (bind _outhits (Collision|MultiSphereTraceForObjects _returnvalue _returnvalue (Variables|Default|GetDamageRadius) (Utilities|Array|MakeArray "ObjectTypeQuery9") false (Utilities|Array|MakeArray EnemyHit) "ForOneFrame"))
    (for _array_element _outhits
      (Game|SpawnActorfromClass "VirusProjectileBP_C" (Math|Transform|MakeTransform (.Location (Collision|BreakHitResult _array_element)) (Math|Rotator|FindLookatRotation (.Location (Collision|BreakHitResult _array_element)) (.ImpactPoint (Collision|BreakHitResult _array_element)))) "AdjustIfPossibleButAlwaysSpawn" 0 (+ (Variables|Default|GetIteration) 1) 1.0 0))))