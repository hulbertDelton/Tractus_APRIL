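; Coil turret projectile that explodes on damaging an enemy, dealing area damage and a brief stun.
; It attaches a fire effect on BeginPlay and overrides the parent's DamageEnemy event to apply both within DamageRadius.
; ApplyRadialStun sphere-traces one object type and sends StunMessage to each hit actor, while radial damage applies at full strength.
; Each impact also spawns an explosion effect and sound, and draws a debug circle of the radius.
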(event EventBeginPlay
  (|CallParentFunction)
  (Effects|SpawnEmitterAttached "/Game/VFX/weaponEffects/coil/coil_fireVFX_ver01.coil_fireVFX_ver01" (Variables|Default|GetBox) "None"))

(event Collision|EventActorBeginOverlap
  (params (OtherActor :type Actor%20Object%20Reference))
  (|CallParentFunction OtherActor) ; This node is disabled and will not be called.\nDrag off pins to build functionality.
)

(event EventTick
  (params (DeltaSeconds :type Float%20%28single-precision%29))
  (|CallParentFunction DeltaSeconds) ; This node is disabled and will not be called.\nDrag off pins to build functionality.
)

(event EventDamageEnemy
  (params (DamagedActor :type Actor%20Object%20Reference))
  (bind _returnvalue (Transformation|GetActorTransform))
  (bind _self self)
  (bind _damageradius (Variables|Default|GetDamageRadius))
  (bind _returnvalue_2 (Transformation|GetActorLocation _self))
  (bind (_location _rotation) (Math|Transform|BreakTransform _returnvalue))
  (CallFunction|ApplyRadialStun _returnvalue_2 (Variables|Default|GetDamageRadius) 0.1)
  (Rendering|Debug|DrawDebugCircle _returnvalue_2 _damageradius 30 "(R=1.000000,G=1.000000,B=1.000000,A=1.000000)" 0.1 0.0 "0.000000,1.000000,0.000000" "1.000000,0.000000,0.000000")
  (Game|Damage|ApplyRadialDamage (Variables|Default|GetExplosionDamage) _returnvalue_2 _damageradius 0 0 0 0 true "ECC_GameTraceChannel3")
  (|CallParentFunction DamagedActor)
  (bind _returnvalue_3 (Effects|SpawnEmitteratLocation "/Game/VFX/weaponEffects/coil/coil_impactExplosion_FX.coil_impactExplosion_FX" _location _rotation "1.000000,1.000000,1.000000" true "AutoRelease"))
  (Audio|SpawnSoundatLocation "/Game/SFX/TURRETS/COIL/COIL_Hit.COIL_Hit" _location "0, 0, 0" 1.0 1.0 0.0 0 0)
  (Effects|Components|ParticleSystem|SetColorParameter _returnvalue_3 "None" "(R=0.000000,G=0.937138,B=0.989583,A=1.000000)"))

(fn ConstructionScript
  (|CallParentFunction))

(fn ApplyRadialStun
  (params (Origin :type Vector) (Radius :type Float%20%28single-precision%29) (Duration :type Float%20%28single-precision%29))
  (bind _outhits (Collision|MultiSphereTraceForObjects Origin Origin Radius (Utilities|Array|MakeArray "ObjectTypeQuery9") false 0 "None"))
  (for _array_element _outhits
    (Class|TractusDamge|Stun(Message) (.HitActor (Collision|BreakHitResult _array_element)) Duration)))