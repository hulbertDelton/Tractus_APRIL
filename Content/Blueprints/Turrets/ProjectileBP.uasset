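; Turret projectile Blueprint that damages enemies on contact and expires after a set lifespan.
; Its box overlap casts the other actor to EnemyBP and applies damage credited to the instigator's controller.
; Optional knockback passes the projectile movement velocity to the enemy through a KnockbackMessage call.
; Non-piercing projectiles destroy themselves after a hit, while piercing ones keep flying.
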(event OnComponentBeginOverlap(Box)
  (params (OverlappedComponent :type Primitive%20Component%20Object%20Reference) (OtherActor :type Actor%20Object%20Reference) (OtherComp :type Primitive%20Component%20Object%20Reference) (OtherBodyIndex :type Integer) (bFromSweep :type Boolean) (SweepResult :type Hit%20Result%20Structure%20%28by%20ref%29))
  (bind _asenemy_bp (Utilities|Casting|CastToEnemyBP OtherActor))
  (CallFunction|DamageEnemy _asenemy_bp))

(event EventBeginPlay
  (Actor|SetLifeSpan (Variables|Default|Getlifespan)))

(event Collision|EventActorBeginOverlap
  (params (OtherActor :type Actor%20Object%20Reference)))

(event EventTick
  (params (DeltaSeconds :type Float%20%28single-precision%29)))

(fn ConstructionScript)

(fn DamageEnemy
  (params (DamagedActor :type Actor%20Object%20Reference))
  (bind _output_get (LocalVariables|SetEnemyHit DamagedActor))
  (Game|Damage|ApplyDamage _output_get (Variables|Default|GetDamage) (Pawn|GetController (Variables|Actor|GetInstigator)) self)
  (if (Variables|Default|GethasKnockback)
    (bind _knockbackamount (CallFunction|GetKnockback))
    (Class|TractusDamge|Knockback(Message) (LocalVariables|GetEnemyHit) _knockbackamount))
  (if (not (Variables|Default|GetisPiercing))
    (Actor|DestroyActor)))

(fn GetKnockback
  (return (Variables|/Script/Engine.MovementComponent|GetVelocity (Variables|Default|GetProjectileMovement))))