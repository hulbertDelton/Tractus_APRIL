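; Railgun turret Blueprint that defines how the turret fires at a target enemy, relying on inherited turret logic.
; On the fire event it sets the railgun shot sound, then calls ShootProjectile with the railgun projectile class and the turret's projectile damage.
; The shot transform takes its location from the RAILGUN socket on Body and its rotation from the TurretOrientation component.
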(event EventBeginPlay
  (|CallParentFunction) ; This node is disabled and will not be called.\nDrag off pins to build functionality.
)

(event Collision|EventActorBeginOverlap
  (params (OtherActor :type Actor%20Object%20Reference))
  (|CallParentFunction OtherActor) ; This node is disabled and will not be called.\nDrag off pins to build functionality.
)

(event EventTick
  (params (DeltaSeconds :type Float%20%28single-precision%29))
  (|CallParentFunction DeltaSeconds) ; This node is disabled and will not be called.\nDrag off pins to build functionality.
)

(event EventFireatTargetEnemy
  (Variables|Default|SetProjectileSound "/Game/SFX/testingSounds/Turrets/RAILGUN_Shot.RAILGUN_Shot")
  (CallFunction|ShootProjectile (Variables|Default|GetProjectileDamage) "/Game/Blueprints/Turrets/RailgunProjectileBP.RailgunProjectileBP_C" (Math|Transform|MakeTransform (Transformation|GetSocketLocation (Variables|Default|GetBody) "RAILGUN") (Transformation|GetSocketRotation (Variables|Default|GetTurretOrientation) "None")) 0.0))

(fn ConstructionScript
  (|CallParentFunction))