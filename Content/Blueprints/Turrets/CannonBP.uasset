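; Cannon turret Blueprint that fires cannon projectiles at enemy targets.
; On the fire-at-target event it sets the cannon shot sound, then calls ShootProjectile with CannonProjectileBP and a fixed damage value.
; The shot originates at the Body's CANNON socket and takes its rotation from the TurretOrientation component.
; It holds no targeting or tick logic of its own, and its construction script only calls the parent.
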(event EventBeginPlay
  (|CallParentFunction) ; This node is disabled and will not be called.\nDrag off pins to build functionality.
)

(event Collision|EventActorBeginOverlap
  (params (OtherActor :type Actor%20Object%20Reference))
  (|CallParentFunction OtherActor) ; This node is disabled and will not be called.\nDrag off pins to build functionality.
)

(event EventTick
  (params (DeltaSeconds :type Float%20%28single-precision%29))
  (|CallParentFunction DeltaSeconds) ; This node is disabled and will not be called.\nDrag off pins to build functionality.
)

(event EventFireatTargetEnemy
  (Variables|Default|SetProjectileSound "/Game/SFX/testingSounds/Turrets/CANNON_Shot.CANNON_Shot")
  (CallFunction|ShootProjectile 5.0 "/Game/Blueprints/Turrets/CannonProjectileBP.CannonProjectileBP_C" (Math|Transform|MakeTransform (Transformation|GetSocketLocation (Variables|Default|GetBody) "CANNON") (Transformation|GetSocketRotation (Variables|Default|GetTurretOrientation) "None")) 0.0))

(fn ConstructionScript
  (|CallParentFunction))