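; Flak turret Blueprint that fires a multi-projectile burst when its fire-at-target event runs.
; The event sets the shot sound, then calls ShootMultiProjectile to launch FlakProjectileBP with the turret's damage and projectile count at a 360-degree spread.
; The fire origin combines the Body's location with the TurretOrientation component's rotation.
; BeginPlay, overlap and Tick are disabled stubs, and the construction script only calls its parent.
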(event EventBeginPlay
  (|CallParentFunction) ; This node is disabled and will not be called.\nDrag off pins to build functionality.
)

(event Collision|EventActorBeginOverlap
  (params (OtherActor :type Actor%20Object%20Reference))
  (|CallParentFunction OtherActor) ; This node is disabled and will not be called.\nDrag off pins to build functionality.
)

(event EventTick
  (params (DeltaSeconds :type Float%20%28single-precision%29))
  (|CallParentFunction DeltaSeconds) ; This node is disabled and will not be called.\nDrag off pins to build functionality.
)

(event EventFireatTargetEnemy
  (Variables|Default|SetProjectileSound "/Game/SFX/testingSounds/Turrets/SPEAR_Shot.SPEAR_Shot")
  (CallFunction|ShootMultiProjectile (Variables|Default|GetProjectileDamage) "/Game/Blueprints/Turrets/FlakProjectileBP.FlakProjectileBP_C" (Math|Transform|MakeTransform (Transformation|GetSocketLocation (Variables|Default|GetBody) "") (Transformation|GetSocketRotation (Variables|Default|GetTurretOrientation) "None")) (Variables|Default|GetProjectileCount) 3.6e+02))

(fn ConstructionScript
  (|CallParentFunction))