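; Spray turret Blueprint that fires spray projectiles at its target enemy, building on an inherited turret base.
; Its fire event sets the shot sound, then calls ShootProjectile with random spread, taking position from the Body's SPEAR socket and rotation from the turret orientation component.
; A fire particle effect attaches to the Body's SPRAY socket on each shot.
; BeginPlay, overlap and Tick are disabled stubs.
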(event EventBeginPlay
  (|CallParentFunction) ; This node is disabled and will not be called.\nDrag off pins to build functionality.
)

(event Collision|EventActorBeginOverlap
  (params (OtherActor :type Actor%20Object%20Reference))
  (|CallParentFunction OtherActor) ; This node is disabled and will not be called.\nDrag off pins to build functionality.
)

(event EventTick
  (params (DeltaSeconds :type Float%20%28single-precision%29))
  (|CallParentFunction DeltaSeconds) ; This node is disabled and will not be called.\nDrag off pins to build functionality.
)

(event EventFireatTargetEnemy
  (Variables|Default|SetProjectileSound "/Game/SFX/testingSounds/Turrets/SPRAY_Shot.SPRAY_Shot")
  (CallFunction|ShootProjectile (Variables|Default|GetProjectileDamage) "/Game/Blueprints/Turrets/SprayProjectileBP.SprayProjectileBP_C" (Math|Transform|MakeTransform (Transformation|GetSocketLocation (Variables|Default|GetBody) "SPEAR") (Transformation|GetSocketRotation (Variables|Default|GetTurretOrientation) "None")) 3e+01)
  (Effects|SpawnEmitterAttached "/Game/VFX/weaponEffects/spray/spray_fireVFX_ver01.spray_fireVFX_ver01" (Variables|Default|GetBody) "SPRAY"))

(fn ConstructionScript
  (|CallParentFunction))