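; Flak turret projectile Blueprint that adds flak-specific visual and audio effects to an inherited projectile base.
; On BeginPlay it attaches an enlarged fire emitter to its Box component.
; Overlap handling passes straight to the parent, and the DamageEnemy override calls the parent, then spawns a pooled impact emitter and a hit sound at the projectile's location.
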(event EventBeginPlay
  (|CallParentFunction)
  (Effects|SpawnEmitterAttached "/Game/VFX/weaponEffects/flak/flak_FireFX.flak_FireFX" (Variables|Default|GetBox) "None" "0, 0, 0" "0, 0, 0" "4.000000,4.000000,4.000000"))

(event Collision|EventActorBeginOverlap
  (params (OtherActor :type Actor%20Object%20Reference))
  (|CallParentFunction OtherActor))

(event EventTick
  (params (DeltaSeconds :type Float%20%28single-precision%29))
  (|CallParentFunction DeltaSeconds) ; This node is disabled and will not be called.\nDrag off pins to build functionality.
)

(event EventDamageEnemy
  (params (DamagedActor :type Actor%20Object%20Reference))
  (bind _returnvalue (Transformation|GetActorTransform))
  (bind (_location _rotation) (Math|Transform|BreakTransform _returnvalue))
  (|CallParentFunction DamagedActor)
  (Effects|SpawnEmitteratLocation "/Game/VFX/weaponEffects/flak/flak_ImpactFX.flak_ImpactFX" _location _rotation "1.000000,1.000000,1.000000" false "AutoRelease")
  (Audio|SpawnSoundatLocation "/Game/SFX/testingSounds/Turrets/SPEAR_Hit.SPEAR_Hit" _location "0, 0, 0" 1.0 1.0 0.0 0 0))

(fn ConstructionScript)