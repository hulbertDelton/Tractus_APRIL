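; Aegis turret Blueprint that forms a curved barrier of wall panels and knocks back actors that touch it.
; The construction script adds three static mesh panels, using helper functions for angle, planet distance and relative position to place them along an arc.
; On BeginPlay each panel's overlap event binds to AsWall, which sends the overlapping actor a KnockbackMessage with a fixed-strength vector rotated to that panel's facing.
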(event Custom|CustomEvent_0
  (params (OverlappedComponent :type Primitive%20Component%20Object%20Reference) (OtherActor :type Actor%20Object%20Reference) (OtherComp :type Primitive%20Component%20Object%20Reference) (OtherBodyIndex :type Integer) (bFromSweep :type Boolean) (SweepResult :type Hit%20Result%20Structure%20%28by%20ref%29))
  (CallFunction|AsWall OverlappedComponent OtherActor))

(event EventBeginPlay
  (|CallParentFunction)
  (for _array_element (Variables|Default|GetAegisWalls)
    (Collision|BindEventtoOnComponentBeginOverlap _array_element (delegate Custom|CustomEvent_0))))

(event Collision|EventActorBeginOverlap
  (params (OtherActor :type Actor%20Object%20Reference)))

(event EventTick
  (params (DeltaSeconds :type Float%20%28single-precision%29))
  (|CallParentFunction DeltaSeconds) ; This node is disabled and will not be called.\nDrag off pins to build functionality.
)

(fn ConstructionScript
  (bind _distance (Utilities|GetDistfromPlanet))
  (|CallParentFunction)
  (for _index (range -1 1)
    (bind _returnvalue (AddComponent|AddStaticMeshComponent false (Math|Transform|MakeTransform (Math|Vector|MakeVector (.X (Math|Vector|BreakVector (.Location (Math|Transform|BreakTransform (Utilities|GetRelativePosition _index (Utilities|GetAngle _distance) _distance))))) (.Y (Math|Vector|BreakVector (.Location (Math|Transform|BreakTransform (Utilities|GetRelativePosition _index (Utilities|GetAngle _distance) _distance))))) -6e+02) (.Rotation (Math|Transform|BreakTransform (Utilities|GetRelativePosition _index (Utilities|GetAngle _distance) _distance))) (.Scale (Math|Transform|BreakTransform (Utilities|GetRelativePosition _index (Utilities|GetAngle _distance) _distance))))))
    (Utilities|Array|Add (Variables|Default|GetAegisWalls) _returnvalue)))

(fn AsWall
  (params (self2 :type Scene%20Component%20Object%20Reference) (Object :type Object%20Object%20Reference))
  (Class|TractusDamge|Knockback(Message) Object (Math|Vector|RotateVector "5000.000000, 0, 0" (Transformation|GetWorldRotation self2))))