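; VirusBP is a turret Blueprint that fires virus projectiles at enemies.
; It overrides the fire-at-target event to set the SPEAR shot sound, then calls ShootProjectile with the turret's projectile damage and the VirusProjectileBP class.
; Shots spawn from the Body's SPEAR socket, aimed along TurretOrientation and scaled up threefold.
; BeginPlay, overlap, Tick and construction add no logic of their own.
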(event EventBeginPlay
  (|CallParentFunction) ; This node is disabled and will not be called.\nDrag off pins to build functionality.
)

(event Collision|EventActorBeginOverlap
  (params (OtherActor :type Actor%20Object%20Reference))
  (|CallParentFunction OtherActor) ; This node is disabled and will not be called.\nDrag off pins to build functionality.
)

(event EventTick
  (params (DeltaSeconds :type Float%20%28single-precision%29))
  (|CallParentFunction DeltaSeconds) ; This node is disabled and will not be called.\nDrag off pins to build functionality.
)

(event EventFireatTargetEnemy
  (Variables|Default|SetProjectileSound "/Game/SFX/testingSounds/Turrets/SPEAR_Shot.SPEAR_Shot")
  (CallFunction|ShootProjectile (Variables|Default|GetProjectileDamage) "/Game/Blueprints/Turrets/VirusProjectileBP.VirusProjectileBP_C" (Math|Transform|MakeTransform (Transformation|GetSocketLocation (Variables|Default|GetBody) "SPEAR") (Transformation|GetSocketRotation (Variables|Default|GetTurretOrientation) "None") "3.000000,3.000000,3.000000") 0.0))

(fn ConstructionScript
  (|CallParentFunction))