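; Cannon turret projectile Blueprint that turns an enemy hit into an area explosion.
; It overrides DamageEnemy to apply full, non-falloff radial damage around its location, with a trace channel for damage prevention, then calls the parent implementation.
; It also briefly draws a debug circle of the blast radius and spawns a pooled impact explosion effect and hit sound.
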(event EventBeginPlay
  (|CallParentFunction) ; This node is disabled and will not be called.\nDrag off pins to build functionality.
)

(event Collision|EventActorBeginOverlap
  (params (OtherActor :type Actor%20Object%20Reference))
  (|CallParentFunction OtherActor) ; This node is disabled and will not be called.\nDrag off pins to build functionality.
)

(event EventTick
  (params (DeltaSeconds :type Float%20%28single-precision%29))
  (|CallParentFunction DeltaSeconds) ; This node is disabled and will not be called.\nDrag off pins to build functionality.
)

(event EventDamageEnemy
  (params (DamagedActor :type Actor%20Object%20Reference))
  (bind _returnvalue (Transformation|GetActorTransform))
  (bind _self self)
  (bind _damageradius (Variables|Default|GetDamageRadius))
  (bind _returnvalue_2 (Transformation|GetActorLocation _self))
  (bind (_location _rotation) (Math|Transform|BreakTransform _returnvalue))
  (Rendering|Debug|DrawDebugCircle _returnvalue_2 _damageradius 30 "(R=1.000000,G=1.000000,B=1.000000,A=1.000000)" 0.1 0.0 "0.000000,1.000000,0.000000" "1.000000,0.000000,0.000000")
  (Game|Damage|ApplyRadialDamage (Variables|Default|GetExplosionDamage) _returnvalue_2 _damageradius 0 0 0 0 true "ECC_GameTraceChannel3")
  (|CallParentFunction DamagedActor)
  (Effects|SpawnEmitteratLocation "/Game/VFX/weaponEffects/cannon/cannonImpactExplosionVFX.cannonImpactExplosionVFX" _location _rotation "1.000000,1.000000,1.000000" false "AutoRelease")
  (Audio|SpawnSoundatLocation "/Game/SFX/testingSounds/Turrets/CANNON_Hit.CANNON_Hit" _location "0, 0, 0" 1.0 1.0 0.0 0 0))

(fn ConstructionScript
  (|CallParentFunction))