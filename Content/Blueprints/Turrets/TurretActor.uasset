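; Turret actor that tracks overlapping enemies within its range and fires projectiles at them, with a selection highlight and range sprite.
; Each tick it picks a closest enemy, turns toward it at a limited speed and fires, gated by fire rate.
; Aim leads moving targets using projectile speed cached from the last shot.
; Hitscan and multi-projectile spread functions also exist, but the default fire path uses single projectiles.
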(event EventBeginPlay
  (Variables|Default|SetMyMaterial (Rendering|Material|GetMaterial (Variables|Default|GetBody) 0))
  (CallFunction|DeSelect))

(event Collision|EventActorBeginOverlap
  (params (OtherActor :type Actor%20Object%20Reference))
  (bind _asenemy_bp (Utilities|Casting|CastToEnemyBP OtherActor))
  (Utilities|Array|Add (Variables|Default|GetVisibleTargets) _asenemy_bp))

(event EventTick
  (params (DeltaSeconds :type Float%20%28single-precision%29))
  (CallFunction|TargetEnemy))

(event Collision|EventActorEndOverlap
  (params (OtherActor :type Actor%20Object%20Reference))
  (bind _asenemy_bp (Utilities|Casting|CastToEnemyBP OtherActor))
  (Utilities|Array|RemoveItem (Variables|Default|GetVisibleTargets) _asenemy_bp))

(event EventSelect
  (Rendering|Material|SetMaterial (Variables|Default|GetBody) 0 "/Game/Materials/preAlphaMaterials/turretSelectorTextures/turretSelector.turretSelector")
  (Rendering|SetVisibility (Variables|Default|Getsprite) true false))

(event EventDeSelect
  (Rendering|Material|SetMaterial (Variables|Default|GetBody) 0 (Variables|Default|GetMyMaterial))
  (Rendering|SetVisibility (Variables|Default|Getsprite) false false))

(fn ConstructionScript
  (bind _range (Variables|Default|GetRange))
  (bind _returnvalue (AddComponent|AddPaperSpriteComponent false (Math|Transform|MakeTransform "0, 0, 0" "0, 0,90.000000" (Math|Conversions|ToVector(Float) (/ (Variables|Default|GetRange) 5e+02)))))
  (bind _output_get (Variables|Default|Setsprite _returnvalue))
  (Collision|SetCollisionResponsetoChannel _output_get "ECC_GameTraceChannel1" "ECR_Ignore")
  (Variables|/Game/Blueprints/TurningSpeedRateLimits.TurningSpeedRateLimits_C|SetMax%20Angular%20Velocity (Variables|Default|GetTurningSpeedRateLimits) (Variables|Default|GetTurningSpeed))
  (Components|Capsule|SetCapsuleSize (Variables|Default|GetTargetingHitbox) _range _range true)
  (if (<= (Variables|Default|GetFiringSpeed) 0.0)
    (Variables|Default|SetFiringSpeed 1e-05)))

(fn TargetEnemy
  (if (> (Utilities|Array|Length (Variables|Default|GetVisibleTargets)) 0)
    (CallFunction|GetClosestEnemy)
    (CallFunction|FaceTargetEnemy)
    (CallFunction|FireatTargetEnemy)))

(fn GetClosestEnemy
  (bind _visibletargets (Variables|Default|GetVisibleTargets))
  (for (_array_element _array_index) _visibletargets
    (Utilities|IsValid _array_element
      (:Is%20Valid
        (if (<= (Transformation|GetDistanceTo _array_element self) (LocalVariables|Getcurrent%20closest))
          (Variables|Default|SetTarget _array_element)
          (LocalVariables|Setcurrent%20closest (Transformation|GetDistanceTo _array_element self))))
      (:Is%20Not%20Valid
        (Utilities|Array|RemoveIndex _visibletargets _array_index)
        (Development|PrintString "Removed!")))))

(fn FaceTargetEnemy
  (bind _returnvalue (Transformation|GetActorLocation))
  (bind _target (Variables|Default|GetTarget))
  (if (!= (Variables|Default|GetProjectileSpeed) 0.0)
    (Default|Turnto (Variables|Default|GetTurningSpeedRateLimits) (Variables|Default|GetTurretOrientation) (Math|Rotator|FindLookatRotation _returnvalue (+ (Transformation|GetActorLocation _target) (* (Transformation|GetVelocity _target) (/ (Transformation|GetDistanceTo _target) (Variables|Default|GetProjectileSpeed))))))
    (else
      (Default|Turnto (Variables|Default|GetTurningSpeedRateLimits) (Variables|Default|GetTurretOrientation) (Math|Rotator|FindLookatRotation _returnvalue (Transformation|GetActorLocation (Variables|Default|GetTarget)))))))

(fn FireatTargetEnemy
  (bind _turretorientation (Variables|Default|GetTurretOrientation))
  (CallFunction|ShootProjectile 3.0 "/Game/Blueprints/Turrets/ProjectileBP.ProjectileBP_C" (Math|Transform|MakeTransform (Transformation|GetSocketLocation _turretorientation "None") (Transformation|GetSocketRotation _turretorientation "None")) 0.0))

(fn ShootHitscan
  (bind _turretorientation (Variables|Default|GetTurretOrientation))
  (bind _parentplanet (Variables|Default|GetParentPlanet))
  (bind _returnvalue (Transformation|GetSocketLocation _turretorientation "None"))
  (bind _outhits (Class|KismetSystemLibrary|LineTraceMultiforObjects _returnvalue (+ _returnvalue (Math|Vector|RotateVector (Math|Vector|MakeVector (Math|Float|MakeLiteralFloat (Variables|Default|GetRange)) 0.0 0.0) (Transformation|GetWorldRotation (Variables|Default|GetTurretOrientation)))) (Utilities|Array|MakeArray "ObjectTypeQuery9" "ObjectTypeQuery2" "ObjectTypeQuery1" "ObjectTypeQuery8" "ObjectTypeQuery7") false 0 "ForOneFrame" true "(R=1.000000,G=0.000000,B=0.000000,A=1.000000)" "(R=0.000000,G=1.000000,B=0.000000,A=1.000000)" 0.1))
  (for _array_element _outhits
    (Game|Damage|ApplyDamage (.HitActor (Collision|BreakHitResult _array_element)) 1.0 (Pawn|GetController _parentplanet) _parentplanet)))

(fn ShootProjectile
  (params (Damage :type Float%20%28single-precision%29) (ProjectileType :type Projectile%20BP%20Class%20Reference) (FireOrigin :type Transform) (Randomness :type Float%20%28single-precision%29))
  (bind (_location _rotation _scale) (Math|Transform|BreakTransform FireOrigin))
  (LocalVariables|SetDamageLocal Damage)
  (LocalVariables|SetProjectileTypeLocal ProjectileType)
  (Utilities|IsReadytoFire
    (:Ready
      (Audio|SpawnSoundAttached (Variables|Default|GetProjectileSound) (Variables|Default|GetBody) "None" "0, 0, 0" "0, 0, 0" "KeepRelativeOffset" false 1.0 1.0 0.0 0 0)
      (bind _returnvalue (Game|SpawnActorfromClass (LocalVariables|GetProjectileTypeLocal) (Math|Transform|MakeTransform _location (Math|Rotator|CombineRotators _rotation (Math|Rotator|MakeRotator 0.0 0.0 (* Randomness (Math|Random|RandomFloatinRange -1.0 1.0)))) _scale) "AlwaysSpawn" 0 (LocalVariables|GetDamageLocal) (Variables|Default|GetParentPlanet)))
      (Variables|Default|SetProjectileSpeed (Math|Vector|VectorLength (Transformation|GetVelocity _returnvalue))))))

(fn ShootMultiProjectile
  (params (Damage :type Float%20%28single-precision%29) (ProjectileType :type Projectile%20BP%20Class%20Reference) (FireOrigin :type Transform) (Count :type Integer) (Spread :type Float%20%28single-precision%29))
  (bind (_location _rotation _scale) (Math|Transform|BreakTransform FireOrigin))
  (LocalVariables|SetDamageLocal Damage)
  (LocalVariables|SetProjectileTypeLocal ProjectileType)
  (LocalVariables|SetSweepStart (/ (Math|Float|ClampAngle Spread 0.0 3.6e+02) -2.0))
  (Utilities|IsReadytoFire
    (:Ready
      (Audio|SpawnSoundAttached (Variables|Default|GetProjectileSound) (Variables|Default|GetBody) "None" "0, 0, 0" "0, 0, 0" "KeepRelativeOffset" false 1.0 1.0 0.0 0 0)
      (for _index (range 1 Count)
        (bind _returnvalue (Game|SpawnActorfromClass (LocalVariables|GetProjectileTypeLocal) (Math|Transform|MakeTransform _location (Math|Rotator|CombineRotators _rotation (Math|Rotator|MakeRotator 0.0 0.0 (/ (* _index Spread) (Math|Conversions|ToFloat(Integer) Count)))) _scale) "AlwaysSpawn" 0 (LocalVariables|GetDamageLocal) (Variables|Default|GetParentPlanet)))
        (Variables|Default|SetProjectileSpeed (Math|Vector|VectorLength (Transformation|GetVelocity _returnvalue)))))))