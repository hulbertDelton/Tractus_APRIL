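; Ring Blueprint that spins about its yaw axis and carries size, turret count and rotation speed settings.
; Each Tick, Update adds RotationSpeed as relative yaw, unscaled by delta time, then draws a horizontal debug circle of radius Size lasting ten seconds.
; Helpers print the ring's settings and convert an index and count into evenly spaced angles; no turret spawning appears here.
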(event EventBeginPlay)

(event EventTick
  (params (DeltaSeconds :type Float%20%28single-precision%29))
  (CallFunction|Update))

(fn PrintRingBp
  (Development|PrintString (Utilities|String|Append "New ring of Size: [" (Utilities|String|ToString(Float) (Variables|Default|GetSize)) "], #Turrets: [" (Utilities|String|ToString(Integer) (Variables|Default|GetNumTurrets)) "], Rotation:" (Utilities|String|ToString(Float) (Variables|Default|GetRotationSpeed)) "]")))

(fn Draw
  (Rendering|Debug|DrawDebugCircle "0, 0, 0" (Variables|Default|GetSize) 60 "(R=1.000000,G=1.000000,B=1.000000,A=1.000000)" 1e+01 0.0 "0.000000,1.000000,0.000000" "1.000000,0.000000,0.000000"))

(fn Update
  (Transformation|AddRelativeRotation (Math|Rotator|MakeRotator 0.0 0.0 (Variables|Default|GetRotationSpeed)) false false)
  (CallFunction|Draw))

(fn AnglefromIndex
  (params (index :type Integer) (Count :type Integer))
  (return (/ (* index 3.6e+02) (Math|Conversions|ToFloat(Integer) Count))))