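; TurretSocketBase is a base turret socket that can be selected and can hold a single turret.
; Select or button input tints its selection interface blue and sets IsSelected, while deselection restores white.
; AddTurret stores the given turret and hides the selection interface; DestroyTurret destroys that turret and shows the interface again.
; A Render Coords helper draws debug axes at a target's world transform.
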(event Custom|InputFromButton
  (Development|PrintString "Socket Input called")
  (Variables|Default|SetisSelected true)
  (Sprite|SetSpriteColor (Variables|Default|GetOwnedSelectionInterface) "(R=0.000000,G=0.061501,B=1.000000,A=1.000000)"))

(event EventBeginPlay)

(event EventTick
  (params (DeltaSeconds :type Float%20%28single-precision%29)))

(event EventSelect
  (Development|PrintString "Socket Input called")
  (Variables|Default|SetisSelected true)
  (Sprite|SetSpriteColor (Variables|Default|GetOwnedSelectionInterface) "(R=0.000000,G=0.061501,B=1.000000,A=1.000000)"))

(event EventDeSelect
  (Variables|Default|SetisSelected false)
  (Sprite|SetSpriteColor (Variables|Default|GetOwnedSelectionInterface) "(R=1.000000,G=1.000000,B=1.000000,A=1.000000)"))

(fn AddTurret
  (params (Turret :type Turret%20Actor%20Object%20Reference))
  (Variables|Default|SethasTurret true)
  (Variables|Default|SetOwnedTurret Turret)
  (Rendering|SetVisibility (Variables|Default|GetOwnedSelectionInterface) false false))

(fn DestroyTurret
  (Development|PrintString "destroyTurret")
  (Variables|Default|SethasTurret false)
  (Actor|DestroyActor (Variables|Default|GetOwnedTurret))
  (Rendering|SetVisibility (Variables|Default|GetOwnedSelectionInterface) true false))