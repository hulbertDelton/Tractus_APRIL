(event Custom|CloseUI
  (Class|SelectionInterface|DeSelect(Message) (Variables|Default|GetSelectedObject))
  (Rendering|SetVisibility (Variables|Default|GetBuildUIWidget) false false)
  (Rendering|SetVisibility (Variables|Default|GetUpgradeUIWidget) false false)
  (Development|PrintString "Close" true true "(R=1.000000,G=1.000000,B=1.000000,A=1.000000)" 0.25))

(event Custom|DemolishSelectedTurret
  (Development|PrintString "Demo Selected Turret!")
  (Default|DestroyTurret (Variables|Default|GetSelectedObject))
  (CallFunction|CloseUI)
  (Class|SelectionInterface|DeSelect(Message) (Variables|Default|GetSelectedObject)))

(event Custom|UpgradeSelectedTurret
  (Development|PrintString "Upgrade Selected Turret!")
  (CallFunction|CloseUI)
  (Class|SelectionInterface|DeSelect(Message) (Variables|Default|GetSelectedObject)))

(event EventBeginPlay
  (Variables|Default|SetbEnableClickEvents true)
  (bind _outactors (Actor|GetAllActorsOfClass "/Game/Blueprints/Turrets/TurretActor.TurretActor_C"))
  (Variables|Default|SetDebug%20Turret (Utilities|Array|Get(acopy) _outactors))
  (CallFunction|CreateUI)
  (CallFunction|UpdateMoney 0))

(event EventTick
  (params (DeltaSeconds :type Float%20%28single-precision%29)))

(event Input|ActionEvents|InputActionSetName
  (params (Key :type Key%20Structure))
  (:Pressed
    (Development|PrintString "Update NAme!")))

(event Input|MouseEvents|LeftMouseButton
  (params (Key :type Key%20Structure))
  (bind (_hitresult _returnvalue) (Game|Player|GetHitResultUnderCursorbyChannel "TraceTypeQuery3" false))
  (:Pressed
    (if _returnvalue
      (bind _aspaper_sprite_component (Utilities|Casting|CastToPaperSpriteComponent (.HitComponent (Collision|BreakHitResult _hitresult)))
        (:then
          (bind _asturret_socket_base (Utilities|Casting|CastToTurretSocketBase (Transformation|GetAttachParent _aspaper_sprite_component))
            (:then
              (CallFunction|SelectSocket _asturret_socket_base))
            (:CastFailed
              (Class|SelectionInterface|DeSelect(Message) (Variables|Default|GetSelectedObject) :!label _label)
              (CallFunction|CloseUI)
              (Development|PrintString "Click Missed" true true "(R=0.000000,G=0.660000,B=1.000000,A=1.000000)" 1.0))))
        (:CastFailed
          (goto _label))))))

(event Input|MouseEvents|RightMouseButton
  (params (Key :type Key%20Structure)))

(event Custom|Build_Event
  (params (TurretType :type Turret%20Actor%20Class%20Reference))
  (CallFunction|BuyTurret TurretType)
  (Rendering|SetVisibility (Variables|Default|GetBuildUIWidget) false false))

(event Input|ActionEvents|InputActionaddCannon
  (params (Key :type Key%20Structure))
  (:Released
    (CallFunction|BuyTurret "/Game/Blueprints/Turrets/CannonBP.CannonBP_C")))

(event Input|ActionEvents|InputActionaddRailgun
  (params (Key :type Key%20Structure))
  (:Released
    (CallFunction|BuyTurret "/Game/Blueprints/Turrets/RailgunBP.RailgunBP_C")))

(event Input|ActionEvents|InputActionaddAegis
  (params (Key :type Key%20Structure))
  (:Released
    (CallFunction|BuyTurret "/Game/Blueprints/Turrets/AegisBP.AegisBP_C")))

(event Input|ActionEvents|InputActionaddFlak
  (params (Key :type Key%20Structure))
  (:Released
    (CallFunction|BuyTurret "/Game/Blueprints/Turrets/FlakBP.FlakBP_C")))

(event Input|ActionEvents|InputActionaddSpray
  (params (Key :type Key%20Structure))
  (:Released
    (CallFunction|BuyTurret "/Game/Blueprints/Turrets/SprayBP.SprayBP_C")))

(event Input|ActionEvents|InputActionaddSpear
  (params (Key :type Key%20Structure))
  (:Released
    (CallFunction|BuyTurret "/Game/Blueprints/Turrets/SpearBP.SpearBP_C")))

(event Input|ActionEvents|InputActionaddTurret
  (params (Key :type Key%20Structure))
  (:Released
    (CallFunction|BuyTurret "/Game/Blueprints/Turrets/TurretActor.TurretActor_C")))

(event Input|ActionEvents|InputActionaddVirus
  (params (Key :type Key%20Structure))
  (:Released
    (CallFunction|BuyTurret "/Game/Blueprints/Turrets/VirusBP.VirusBP_C")))

(event Input|ActionEvents|InputActionaddCoil
  (params (Key :type Key%20Structure))
  (:Released
    (CallFunction|BuyTurret "/Game/Blueprints/Turrets/CoilBP.CoilBP_C")))

(event Input|ActionEvents|InputActionaddResonator
  (params (Key :type Key%20Structure))
  (:Released
    (CallFunction|BuyTurret "/Game/Blueprints/Turrets/ResonatorBP.ResonatorBP_C")))

(event Input|ActionEvents|InputActionaddIon
  (params (Key :type Key%20Structure))
  (:Released
    (CallFunction|BuyTurret "/Game/Blueprints/Turrets/IonBP.IonBP_C")))

(fn ConstructionScript)

(fn CreateUI
  (Variables|Default|SetbShowMouseCursor true)
  (Class|PlayerController|ClientSetHUD "/Game/UserInterface/TractusV1_HUD.TractusV1_HUD_C")
  (bind _astractus_v1_hud (Utilities|Casting|CastToTractusV1_HUD (HUD|GetHUD)))
  (Variables|Default|SetHUD _astractus_v1_hud)
  (CallFunction|CloseUI))

(fn UpdateMoney
  (params (toAdd :type Integer))
  (bind _output_get (Variables|Default|SetMoney (+ toAdd (Variables|Default|GetMoney))))
  (Default|SetMoney (Variables|Default|GetHUD) _output_get))

(fn CreateTurretfromSocket
  (params (NewParam :type Turret%20Actor%20Class%20Reference))
  (bind _returnvalue (Pawn|GetControlledPawn))
  (LocalVariables|SetTurretType NewParam)
  (if (Utilities|IsValid (Variables|Default|GetSelectedObject))
    (if (not (Variables|/Game/Blueprints/TurretSocketBase.TurretSocketBase_C|GethasTurret (Variables|Default|GetSelectedObject)))
      (if (== (LocalVariables|GetTurretType) "/Game/Blueprints/Turrets/SatelliteBP.SatelliteBP_C")
        (Development|PrintString "TODO in Create turret from socket make sure you can't recuse satellites"))
      (bind _output_get (LocalVariables|SetSocketTransform (Transformation|GetRelativeTransform (Variables|Default|GetSelectedObject))))
      (bind _asdemo_planet_bp (Utilities|Casting|CastToDemoPlanetBP _returnvalue)
        (:then
          (bind _returnvalue_2 (Game|SpawnActorfromClass (LocalVariables|GetTurretType) (Math|Transform|MakeTransform "0, 0, 0" "0, 0, 0" "0.500000,0.500000,0.500000") "AlwaysSpawn" 0 _asdemo_planet_bp "/Game/Blueprints/Turrets/ProjectileBP.ProjectileBP_C" 1.0 _returnvalue))
          (Transformation|AttachComponentToComponent (Variables|/Script/Engine.Actor|GetRootComponent _returnvalue_2) (Variables|Default|GetSelectedObject) "None" "KeepRelative" "KeepRelative" "KeepWorld" false)
          (Default|AddTurret (Variables|Default|GetSelectedObject) _returnvalue_2))
        (:CastFailed
          (Development|PrintString "Cast to demo planet failed"))))
    (else
      (return false))))

(fn BuyTurret
  (params (type_to_build :type Turret%20Actor%20Class%20Reference))
  (bind _output_get (LocalVariables|SetTurretType type_to_build))
  (LocalVariables|SetTurretPrice (.Cost (Utilities|GetClassDefaults _output_get)))
  (LocalVariables|SetProjectileType (.ProjectileType (Utilities|GetClassDefaults _output_get)))
  (if (>= (Variables|Default|GetMoney) (LocalVariables|GetTurretPrice))
    (bind _succeeded (CallFunction|CreateTurretfromSocket (LocalVariables|GetTurretType)))
    (if _succeeded
      (CallFunction|UpdateMoney (- 0 (LocalVariables|GetTurretPrice)))
      (Development|PrintString (Utilities|String|Append "Purchased: " (Utilities|GetClassDisplayName (LocalVariables|GetTurretType))) true true "(R=0.150000,G=0.500000,B=0.000000,A=1.000000)"))
    (else
      (Development|PrintString (Utilities|String|Append "Not Enough Money!: " (Utilities|String|ToString(Integer) (Variables|Default|GetMoney)))))))

(fn SelectTurret
  (params (NewSelection :type Turret%20Socket%20Base%20Object%20Reference))
  (Class|SelectionInterface|DeSelect(Message) (Variables|Default|GetSelectedObject))
  (bind _output_get (Variables|Default|SetSelectedObject NewSelection))
  (Class|SelectionInterface|Select(Message) _output_get)
  (Development|PrintString (Utilities|GetDisplayName _output_get))
  (Rendering|SetVisibility (Variables|Default|GetUpgradeUIWidget) true false))

(fn SelectSocket
  (params (NewParam :type Turret%20Socket%20Base%20Object%20Reference))
  (Class|SelectionInterface|DeSelect(Message) (Variables|Default|GetSelectedObject))
  (Development|PrintString "here select socket")
  (bind _output_get (Variables|Default|SetSelectedObject NewParam))
  (Class|SelectionInterface|Select(Message) _output_get)
  (Development|PrintString (Utilities|GetDisplayName _output_get))
  (bind _asturret_socket_base (Utilities|Casting|CastToTurretSocketBase (Variables|Default|GetSelectedObject)))
  (if (Variables|/Game/Blueprints/TurretSocketBase.TurretSocketBase_C|GethasTurret _asturret_socket_base)
    (Rendering|SetVisibility (Variables|Default|GetUpgradeUIWidget) true false)
    (else
      (Rendering|SetVisibility (Variables|Default|GetBuildUIWidget) true false))))