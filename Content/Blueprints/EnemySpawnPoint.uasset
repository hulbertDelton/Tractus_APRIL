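; Enemy spawner actor that creates single enemies and enemy formations around the world origin on looping timers.
; BeginPlay starts one timer for SpawnGenericEnemy, which places EnemyType at a random angle and distance in a ring around the origin.
; A second timer runs SpawnOppositeSpirals, spawning two EnemyFormationBPOld formations with random yaws from opposite half-circles.
; SpawnSymphony combines a single enemy with two one-unit formations, but nothing here calls it.
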(event EventBeginPlay
  (bind _returnvalue (Utilities|Time|SetTimerbyFunctionName self "SpawnGenericEnemy" (Variables|Default|GetSpawnTimerInterval) true))
  (Variables|Default|SetSpawnGenericTimerHandle _returnvalue)
  (Utilities|Time|SetTimerbyFunctionName 0 "SpawnOppositeSpirals" 3.0 true))

(event Collision|EventActorBeginOverlap
  (params (OtherActor :type Actor%20Object%20Reference)))

(event EventTick
  (params (DeltaSeconds :type Float%20%28single-precision%29)))

(fn ConstructionScript)

(fn SpawnGenericEnemy
  (bind _returnvalue (Game|SpawnActorfromClass (Variables|Default|GetEnemyType) (Math|Transform|MakeTransform (Math|Vector|RotateVector (Math|Vector|MakeVector (Math|Random|RandomFloatinRange 1e+03 1.5e+03) 0.0 0.0) (Math|Rotator|MakeRotator 0.0 0.0 (Math|Random|RandomFloatinRange 0.0 3.6e+02)))) "AdjustIfPossibleButAlwaysSpawn" 0 self))
  (Actor|Tick|SetActorTickEnabled _returnvalue true))

(fn SpawnSymphony
  (bind _returnvalue (Math|Random|RandomFloatinRange 0.0 1.8e+02))
  (Utilities|FlowControl|Sequence
    (:then_0
      (CallFunction|SpawnGenericEnemy)
      (Development|PrintString "1"))
    (:then_1
      (CallFunction|SpawnFormation 1 (Math|Rotator|MakeRotator 0.0 0.0 _returnvalue)))
    (:then_2
      (CallFunction|SpawnFormation 1 (Math|Rotator|MakeRotator 0.0 0.0 (+ _returnvalue 1.8e+02))))))

(fn SpawnFormation
  (params (Units :type Integer) (Rotation :type Rotator))
  (Game|SpawnActorfromClass "/Game/Blueprints/Enemies/EnemyFormationBPOld.EnemyFormationBPOld_C" (Math|Transform|MakeTransform "0, 0, 0" Rotation) "Undefined" 0 Units 0 0))

(fn SpawnOppositeSpirals
  (bind _returnvalue (Math|Random|RandomFloatinRange 0.0 1.8e+02))
  (Utilities|FlowControl|Sequence
    (:then_0
      (CallFunction|SpawnFormation 5 (Math|Rotator|MakeRotator 0.0 0.0 _returnvalue)))
    (:then_1
      (CallFunction|SpawnFormation 5 (Math|Rotator|MakeRotator 0.0 0.0 (+ _returnvalue 1.8e+02))))))