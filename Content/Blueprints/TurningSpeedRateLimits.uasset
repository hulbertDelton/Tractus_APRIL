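; Blueprint that rotates a given component toward a target rotation with a capped turn step.
; TurnTo snaps to the target when the rotator delta's magnitude is within MaxAngularVelocity, otherwise adds that delta scaled to the limit as relative rotation.
; GetRotatorMagnitude treats roll, pitch and yaw as a vector length; the cap applies per call, without delta time.
; SetInterpRotation is an empty stub.
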(event EventBeginPlay)

(event EventTick
  (params (DeltaSeconds :type Float%20%28single-precision%29)))

(fn Turnto
  (params (RotationTarget :type Scene%20Component%20Object%20Reference) (TargetPosition :type Rotator))
  (bind _returnvalue (Transformation|GetWorldRotation RotationTarget))
  (bind _max_angular_velocity (Variables|Default|GetMax%20Angular%20Velocity))
  (bind _returnvalue_2 (Math|Rotator|Delta(Rotator) TargetPosition _returnvalue))
  (bind _magnitude (CallFunction|GetRotatorMagnitude _returnvalue_2))
  (if (!= _magnitude 0.0)
    (LocalVariables|Setrotationtargetlocal RotationTarget)
    (if (<= _magnitude _max_angular_velocity)
      (Transformation|SetWorldRotation (LocalVariables|Getrotationtargetlocal) TargetPosition false false)
      (else
        (Transformation|AddRelativeRotation (LocalVariables|Getrotationtargetlocal) (* _returnvalue_2 (/ _max_angular_velocity _magnitude)) false false)))))

(fn GetRotatorMagnitude
  (params (NewParam :type Rotator%20%28by%20ref%29))
  (bind (_roll _pitch _yaw) (Math|Rotator|BreakRotator NewParam))
  (return (Math|Float|Sqrt (+ (Math|Float|Square _roll) (Math|Float|Square _pitch) (Math|Float|Square _yaw)))))

(fn SetInterpRotation
  (params (RotationTarget :type Scene%20Component%20Object%20Reference) (TargetPosition :type Rotator)))