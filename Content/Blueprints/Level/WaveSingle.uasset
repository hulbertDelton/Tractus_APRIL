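; WaveSingle is a behavior tree task that runs one wave of a level.
; On execute it spawns a formation actor of WaveType, passing in PathColor.
; A Tick state machine polls the formation's CheckForExit, destroys it on exit, waits PostWaveDelay, then finishes the task successfully.
; Print strings log the numbered wave's start and completion.
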(event Custom|Finish%20LEvel
  (Utilities|FlowControl|Delay (Variables|Default|GetPost-Wave%20Delay))
  (Variables|Default|SetState 2))

(event EventReceiveExecute
  (params (OwnerActor :type Actor%20Object%20Reference))
  (Development|PrintString (Utilities|String|Append "Wave " (Utilities|String|ToString(Integer) (Variables|Default|GetWave%20Number)) ": Begin"))
  (Variables|Default|SetState 0)
  (bind _returnvalue (Game|SpawnActorfromClass (Variables|Default|GetWave%20type) (Math|Transform|MakeTransform "0, 0, 0") "Undefined" 0 10 0 (Variables|Default|GetPathColor) 0))
  (Variables|Default|SetFormation _returnvalue))

(event EventTick
  (params (OwnerActor :type Actor%20Object%20Reference) (DeltaSeconds :type Float%20%28single-precision%29))
  (switch int (Variables|Default|GetState)
    (:0
      (bind _isdone (Default|CheckforExit (Variables|Default|GetFormation)))
      (if _isdone
        (Development|PrintString "Behavior Tree observed wave completion")
        (Variables|Default|SetState 1)
        (Development|PrintString (Utilities|String|Append "Wave " (Utilities|String|ToString(Integer) (Variables|Default|GetWave%20Number)) ": Complete!"))
        (Actor|DestroyActor (Variables|Default|GetFormation))))
    (:1
      (CallFunction|FinishLEvel))
    (:2
      (AI|BehaviorTree|FinishExecute true))))