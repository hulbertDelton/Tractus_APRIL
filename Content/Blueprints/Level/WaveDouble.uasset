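; Behavior Tree task that runs a two-formation enemy or unit wave and finishes once it completes.
; On execute it spawns differently colored formations from two configurable classes, though Formation2 is set to None rather than the second spawn.
; Tick drives a small state machine: poll both formations' CheckForExit, destroy them when both pass, wait a post-wave delay, then finish the task successfully.
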(event Custom|Finish%20LEvel
  (Utilities|FlowControl|Delay (Variables|Default|GetPost-Wave%20Delay))
  (Variables|Default|SetState 2))

(event EventReceiveExecute
  (params (OwnerActor :type Actor%20Object%20Reference))
  (bind _returnvalue (Math|Transform|MakeTransform "0, 0, 0"))
  (Development|PrintString (Utilities|String|Append "Wave " (Utilities|String|ToString(Integer) (Variables|Default|GetWave%20Number)) ": Begin"))
  (Variables|Default|SetState 0)
  (bind _returnvalue_2 (Game|SpawnActorfromClass (Variables|Default|GetWaveTypeFirst) _returnvalue "Undefined" 0 30 0 "(R=0.000000,G=0.078688,B=1.000000,A=1.000000)" 0))
  (Variables|Default|SetFormation _returnvalue_2)
  (Game|SpawnActorfromClass (Variables|Default|GetWaveTypeSecond) _returnvalue "Undefined" 0 30 0 "(R=1.000000,G=0.176995,B=0.000000,A=1.000000)" 0)
  (Variables|Default|SetFormation2 0))

(event EventTick
  (params (OwnerActor :type Actor%20Object%20Reference) (DeltaSeconds :type Float%20%28single-precision%29))
  (switch int (Variables|Default|GetState)
    (:0
      (bind _isdone (Default|CheckforExit (Variables|Default|GetFormation)))
      (bind _isdone_2 (Default|CheckforExit (Variables|Default|GetFormation2)))
      (if (and _isdone_2 _isdone)
        (Development|PrintString "Behavior Tree observed wave completion")
        (Variables|Default|SetState 1)
        (Development|PrintString (Utilities|String|Append "Wave " (Utilities|String|ToString(Integer) (Variables|Default|GetWave%20Number)) ": Complete!"))
        (Actor|DestroyActor (Variables|Default|GetFormation))
        (Actor|DestroyActor (Variables|Default|GetFormation2))))
    (:1
      (CallFunction|FinishLEvel))
    (:2
      (AI|BehaviorTree|FinishExecute true))))